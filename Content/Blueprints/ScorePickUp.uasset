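; A pooled score pickup that awards points to a ThirdPersonCharacter when its static mesh is hit.
; The hit disables mesh collision, then checks that the other actor has a CharacterMovementComponent.
; The player character is looked up through the PlayerIndex of that actor's MotionControllerComponent.
; The character's score-increment dispatcher receives Pickable, PoolChild returns the pickup to its pool, and the character triggers an item respawn.
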(event OnComponentHit(StaticMesh)
  (params (HitComponent :type Primitive%20Component%20Object%20Reference) (OtherActor :type Actor%20Object%20Reference) (OtherComp :type Primitive%20Component%20Object%20Reference) (NormalImpulse :type Vector :default "0, 0, 0") (Hit :type Hit%20Result%20Structure%20%28by%20ref%29))
  ;[1 1 1] Set visibility false on component hit
  (Collision|SetCollisionEnabled (Variables|Default|GetStaticMesh) "NoCollision")
  (Utilities|IsValid (Actor|GetComponentbyClass OtherActor "/Script/Engine.CharacterMovementComponent")
    (:Is%20Valid
      (bind _asthird_person_character (Utilities|Casting|CastToThirdPersonCharacter (Game|GetPlayerCharacter (Variables|/Script/HeadMountedDisplay.MotionControllerComponent|GetPlayerIndex (Actor|GetComponentbyClass OtherActor "/Script/HeadMountedDisplay.MotionControllerComponent")))))
      (Default|CallIncrementScoreED _asthird_person_character (Variables|Default|GetPickable))
      (Class|PoolChild|ReturntoPool (Variables|Default|GetPoolChild))
      (Default|CallRespawnItem _asthird_person_character))))

(event EventBeginPlay)

(event Collision|EventActorBeginOverlap
  (params (OtherActor :type Actor%20Object%20Reference)))

(event EventTick
  (params (DeltaSeconds :type Float%20%28single-precision%29)))

(fn ConstructionScript)